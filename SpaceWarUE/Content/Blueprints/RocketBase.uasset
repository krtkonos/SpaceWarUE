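; Base rocket Blueprint providing functions for physics-driven flight, fuel use, shooting and explosive destruction, with no event logic of its own.
; Velocity-change impulses drive capped rotation and fuel-gated thrust along the mesh's up vector, while VeilPull pulls components toward the world origin.
; FireFnc launches ammo-limited projectiles, and DestroyAndExplode spawns an explosion effect.
; Helpers test screen bounds and horizontal distance from the origin, and pick random positions away from the center.
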(fn `CheckDistance`
  (params (Mesh :type "MeshComponent Object Reference"))
  (returns (ShouldDestroy :type Boolean))
  (bind (_returnvalue_x _returnvalue_y _returnvalue_z) (`KismetMathLibrary.BreakVector` (`SceneComponent.K2_GetComponentLocation` Mesh)))
  (bind _returnvalue (`KismetMathLibrary.Vector_Distance` (`KismetMathLibrary.MakeVector` 0.0 0.0 _returnvalue_z) (`SceneComponent.K2_GetComponentLocation` Mesh)))
  (return (or (< _returnvalue (`self.MinimalDistance`)) (> _returnvalue (`self.MaximalDistance`)))))

(fn `DestroyAndExplode`
  (params (Transform :type "Transform Structure"))
  (`self.K2_DestroyActor`)
  (`|SpawnActorFromClass` "/Game/StarterContent/Blueprints/Blueprint_Effect_Explosion.Blueprint_Effect_Explosion_C" Transform "Undefined" "OverrideRootScale" null null))

(fn `DestroyIfOffScreen`
  (params (Position :type "Vector Structure") (Mesh :type "MeshComponent Object Reference"))
  (returns (ReturnValue :type Boolean))
  (bind (_returnvalue_x _returnvalue_y) (`KismetMathLibrary.BreakVector2D` (`WidgetLayoutLibrary.GetViewportSize`)))
  (bind _screenlocation (`PlayerController.ProjectWorldLocationToScreen` (`GameplayStatics.GetPlayerController` 0) (`SceneComponent.K2_GetComponentLocation` Mesh) false))
  (return (and (> (`KismetMathLibrary.BreakVector2D` _screenlocation) 0.0) (> (`.Y` (`KismetMathLibrary.BreakVector2D` _screenlocation)) 0.0) (< (`KismetMathLibrary.BreakVector2D` _screenlocation) _returnvalue_x) (< (`.Y` (`KismetMathLibrary.BreakVector2D` _screenlocation)) _returnvalue_y))))

(fn `FireFnc`
  (params (SpawnTransform :type "Transform Structure"))
  (if (> (`self.AmmoCount`) 0)
    (bind _returnvalue (`|SpawnActorFromClass` "/Game/StarterContent/Blueprints/BP_Projectile.BP_Projectile_C" SpawnTransform "Undefined" "OverrideRootScale" null null))
    (`PrimitiveComponent.AddImpulse` (`StaticMeshActor.StaticMeshComponent` _returnvalue) (* (`self.GetActorForwardVector` _returnvalue) 1000.0) "None" true)
    (bind _result (`/Engine/EditorBlueprintResources/StandardMacros.DecrementInt` (`self.AmmoCount`))
      (:`  `
        (set `self.AmmoCount` _result)))))

(fn `Get Accelerate`
  (params (Mesh :type "MeshComponent Object Reference"))
  (returns (ReturnValue :type Boolean))
  (bind _returnvalue (> (`self.Fuel`) 0))
  (`self.UseFuel`)
  (if (`self.Accelerate`)
    (bind _result (`/Engine/EditorBlueprintResources/StandardMacros.IncrementFloat` (`self.AccelerateVelocity`))
      (:`  `
        (bind _output_get (set `self.CurrentImpulse` _result))
        (if (< _output_get (`self.MaxAccelerateVelocity`))
          (if _returnvalue
            (`PrimitiveComponent.AddImpulse` Mesh (* (`KismetMathLibrary.GetUpVector` (`SceneComponent.K2_GetComponentRotation` Mesh)) (`self.AccelerateVelocity`)) "None" true)
            (return _returnvalue)))))
    (elif (> (`self.CurrentImpulse`) 0.0)
      (bind _result_2 (`/Engine/EditorBlueprintResources/StandardMacros.DecrementFloat` (`self.AccelerateVelocity`))
        (:`  `
          (set `self.CurrentImpulse` _result_2))))))

(fn `GetRotateLeft`
  (params (Mesh :type "MeshComponent Object Reference") (Direction :type "Float (double-precision)") (RotBool :type Boolean))
  (bind (_returnvalue_x _returnvalue_y _returnvalue_z) (`KismetMathLibrary.BreakVector` (`PrimitiveComponent.GetPhysicsAngularVelocityInDegrees` Mesh "None")))
  (if RotBool
    (if (> _returnvalue_z (* (`self.MaxRStrength`) -1.0))
      (`PrimitiveComponent.AddAngularImpulseInDegrees` Mesh (`KismetMathLibrary.MakeVector` 0.0 0.0 (* (`self.RotateStrength`) -1.0)) "None" true)
      (return))))

(fn `GetRotateRight`
  (params (ShouldRotate :type Boolean) (Mesh :type "MeshComponent Object Reference"))
  (bind (_returnvalue_x _returnvalue_y _returnvalue_z) (`KismetMathLibrary.BreakVector` (`PrimitiveComponent.GetPhysicsAngularVelocityInDegrees` Mesh "None")))
  (if ShouldRotate
    (if (< _returnvalue_z (`self.MaxRStrength`))
      (`PrimitiveComponent.AddAngularImpulseInDegrees` Mesh (`KismetMathLibrary.MakeVector` 0.0 0.0 (`self.RotateStrength`)) "None" true)
      (return))))

(fn `RandomPoistion`
  (returns (X :type "Float (double-precision)") (Y :type "Float (double-precision)") (Z :type "Float (double-precision)"))
  (return (`KismetMathLibrary.Conv_IntToDouble` (`KismetMathLibrary.SelectInt` (`KismetMathLibrary.RandomIntegerInRange` -600 -220) (`KismetMathLibrary.RandomIntegerInRange` 220 600) (`KismetMathLibrary.RandomBool`))) (`KismetMathLibrary.Conv_IntToDouble` (`KismetMathLibrary.SelectInt` (`KismetMathLibrary.RandomIntegerInRange` -1700 -220) (`KismetMathLibrary.RandomIntegerInRange` 220 1700) (`KismetMathLibrary.RandomBool`))) (`KismetMathLibrary.Conv_IntToDouble` (`KismetMathLibrary.RandomIntegerInRange` 0 360))))

(fn `UseFuel`
  (if (`self.Accelerate`)
    (bind _result (`/Engine/EditorBlueprintResources/StandardMacros.DecrementInt` (`self.Fuel`))
      (:`  `
        (set `self.Fuel` _result)))))

(fn `UserConstructionScript`)

(fn `VeilPull`
  (params (NewParam :type "MeshComponent Object Reference"))
  (if (`KismetSystemLibrary.IsValid` NewParam)
    (`PrimitiveComponent.AddImpulse` NewParam (* (`KismetMathLibrary.Normal` (- (0.0 0.0 0.0) (`SceneComponent.K2_GetComponentLocation` NewParam))) (`self.GravityStrenght`)) "None" true)
    (return)))