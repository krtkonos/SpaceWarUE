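; Eastern R-77 missile projectile Blueprint that exposes control events for its thruster effect and animated fins.
; On BeginPlay it caches the skeletal mesh's Animation Blueprint instance, which the fin events write to directly.
; Normalized inputs are clamped and remapped to degrees, deflecting each of the four fins individually and folding all four together.
; A separate event switches the thruster FX on or off.
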(event `self.ReceiveBeginPlay`
  (bind _asabp_east_missile_r77 (cast `/Game/VigilanteContent/Projectiles/East_Missile_R77/ABP_East_Missile_R77` (`SkeletalMeshComponent.GetAnimInstance` (`self.SkeletalMesh`))))
  (set `self.AnimInstance` _asabp_east_missile_r77))

(event `SetEngineState`
  (params (bEngineActive :type Boolean))
  ;[1 1 1] Set engine state
  (`ActorComponent.SetActive` (`self.ThrusterFX`) bEngineActive true))

(event `SetFin1Angle`
  (params (Angle :type "Float (double-precision)"))
  (set `/Game/VigilanteContent/Projectiles/East_Missile_R77/ABP_East_Missile_R77.Fin1Angle` (`KismetMathLibrary.MapRangeClamped` Angle -1.0 1.0 -45.0 45.0) (`self.AnimInstance`)))

(event `SetFin2Angle`
  (params (Angle :type "Float (double-precision)"))
  (set `/Game/VigilanteContent/Projectiles/East_Missile_R77/ABP_East_Missile_R77.Fin2Angle` (`KismetMathLibrary.MapRangeClamped` Angle -1.0 1.0 -45.0 45.0) (`self.AnimInstance`)))

(event `SetFin3Angle`
  (params (Angle :type "Float (double-precision)"))
  (set `/Game/VigilanteContent/Projectiles/East_Missile_R77/ABP_East_Missile_R77.Fin3Angle` (`KismetMathLibrary.MapRangeClamped` Angle -1.0 1.0 -45.0 45.0) (`self.AnimInstance`)))

(event `SetFin4Angle`
  (params (Angle :type "Float (double-precision)"))
  (set `/Game/VigilanteContent/Projectiles/East_Missile_R77/ABP_East_Missile_R77.Fin4Angle` (`KismetMathLibrary.MapRangeClamped` Angle -1.0 1.0 -45.0 45.0) (`self.AnimInstance`)))

(event `SetFinsFold`
  (params (Angle :type "Float (double-precision)"))
  (bind _animinstance (`self.AnimInstance`))
  (bind _output_get (set `/Game/VigilanteContent/Projectiles/East_Missile_R77/ABP_East_Missile_R77.Fin1Fold` (`KismetMathLibrary.MapRangeClamped` Angle 0.0 1.0 0.0 90.0) _animinstance))
  (bind _output_get_2 (set `/Game/VigilanteContent/Projectiles/East_Missile_R77/ABP_East_Missile_R77.Fin2Fold` _output_get _animinstance))
  (bind _output_get_3 (set `/Game/VigilanteContent/Projectiles/East_Missile_R77/ABP_East_Missile_R77.Fin3Fold` _output_get_2 _animinstance))
  (set `/Game/VigilanteContent/Projectiles/East_Missile_R77/ABP_East_Missile_R77.Fin4Fold` _output_get_3 _animinstance))

(fn `UserConstructionScript`)